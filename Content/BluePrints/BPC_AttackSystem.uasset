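; Attack component for BP_MainCharacter that runs left-click weapon combos and melee hit detection.
; Attack input plays the main weapon's next DataTable montage; presses mid-attack are buffered until 攻击结束, which otherwise resets the combo after a delay.
; Timer-looped sphere traces along the sword damage "harm"-tagged actors with shake, blood and sound, throttled by a DoOnce.
; Charge attacks are stubbed, and the foot trace only draws debug.
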(event `self.ReceiveBeginPlay`
  (bind _asbp_main_character (cast `/Game/ThirdPerson/Blueprints/BP_MainCharacter` (`self.GetOwner`)))
  (set `self.Main_character` _asbp_main_character))

(event `攻击结束`
  (bind _maincharacterstatus (`/Game/ThirdPerson/Blueprints/BP_MainCharacter.MainCharacterStatus` (`self.Main_character`)))
  (set `self.PlayKeyAnimEnd` true)
  (setmembers `/Game/BluePrints/Struct/Struct_CharacterStatus` :`StructRef` _maincharacterstatus :`武器攻击` false)
  (if (`self.Lift_save`)
    (set `self.Lift_save` false)
    (`self.左键武器攻击` 0)
    (else
      (`KismetSystemLibrary.RetriggerableDelay` 0.5)
      (if (not (`.武器攻击_60_D83A8A1B458D968D4F84F5B10B6F9416` (break `/Game/BluePrints/Struct/Struct_CharacterStatus` _maincharacterstatus)))
        (`self.重置攻击`)))))

(event `重置攻击`
  (setmembers `/Game/BluePrints/Struct/Struct_CharacterStatus` :`StructRef` (`/Game/ThirdPerson/Blueprints/BP_MainCharacter.MainCharacterStatus` (`self.Main_character`)) :`武器攻击` false)
  (set `self.Lift_num` 0)
  (set `self.Lift_save` false))

(event `步行环境左键攻击`
  (bind (`_环境` `_步行状态` `_骑马状态` `_主武器`) (break `/Game/BluePrints/Struct/Struct_CharacterStatus` (`/Game/ThirdPerson/Blueprints/BP_MainCharacter.MainCharacterStatus` (`self.Main_character`))))
  (switch `/Game/BluePrints/Struct/Enum_ActiveLand` `_步行状态`
    (:`NewEnumerator0`
      _)
    (:`NewEnumerator1`
      _)
    (:`NewEnumerator2`
      _)
    (:`NewEnumerator3`
      _))
  (bind _returnvalue (`|GetDataTableRow` (`self.DT_Arms_Anim`) (`KismetStringLibrary.Conv_StringToName` (`|GetEnumeratorNameAsString` `_主武器`)))
    (:`then`
      (bind _liftcombo (break `/Game/BluePrints/Data/BPStruct_Arms_Anim` _returnvalue))
      (`|PlayMontage` (`Character.Mesh` (`self.Main_character`)) (`|GetArrayItem` _liftcombo (`self.Lift_num`))
        (:`then`
          (bind _result (`/Engine/EditorBlueprintResources/StandardMacros.IncrementInt` (`self.Lift_num`))
            (:`  `
              (if (>= _result (`KismetArrayLibrary.Array_Length` _liftcombo))
                (set `self.Lift_num` 0)))))
        (:`OnCompleted`
          (set `self.PlayKeyAnimEnd` false :!label _label))
        (:`OnInterrupted`
          (if (`self.PlayKeyAnimEnd`)
            (goto _label)
            (else
              (`self.重置攻击`))))))))

(event `左键武器攻击`
  (params (`蓄力等级` :type Integer))
  (bind _main_character (`self.Main_character`))
  (bind _maincharacterstatus (`/Game/ThirdPerson/Blueprints/BP_MainCharacter.MainCharacterStatus` _main_character))
  (bind (`_环境` `_步行状态` `_骑马状态` `_主武器` `_武器攻击`) (break `/Game/BluePrints/Struct/Struct_CharacterStatus` _maincharacterstatus))
  (if (> (`KismetArrayLibrary.Array_Length` (`/Game/BluePrints/BPC_EquipmentSystem.CurWeaponSlot` (`/Game/ThirdPerson/Blueprints/BP_MainCharacter.BPC_EquipmentSystem` (`self.Main_character`)))) 0)
    (switch `/Game/BluePrints/Struct/Enum_BasicStatue` (`/Game/ThirdPerson/Blueprints/BP_MainCharacter.BasicStatue` _main_character)
      (:`NewEnumerator0`
        _)
      (:`NewEnumerator1`
        _))
    (if `_武器攻击`
      (set `self.Lift_save` true)
      (else
        (setmembers `/Game/BluePrints/Struct/Struct_CharacterStatus` :`StructRef` _maincharacterstatus :`武器攻击` true)
        (switch `/Game/BluePrints/Struct/Enum_ActionEnv` `_环境`
          (:`NewEnumerator0`
            (`self.步行环境左键攻击`)))))))

(event `蓄力中`)

(event `EnhancedInput|/Game/ThirdPerson/Input/Actions/IA_Attack`
  (params (ActionValue :type Boolean) (ElapsedSeconds :type "Float (double-precision)") (TriggeredSeconds :type "Float (double-precision)") (InputAction :type "InputAction Object Reference" :default "/Game/ThirdPerson/Input/Actions/IA_Attack.IA_Attack"))
  (bind _returnvalue (< TriggeredSeconds 0.3))
  ;[1 1 1] 攻击会依赖按键时长而动态变更，蓄力攻击会覆盖普通攻击
  (:`Triggered`
    (if (not _returnvalue)
      (`self.蓄力中`)))
  (:`Started`
    (`self.左键武器攻击` 0))
  (:`Canceled`
    (if _returnvalue
      _
      (elif (> TriggeredSeconds 1.0)
        (`self.左键武器攻击` 0)
        (else
          (`self.左键武器攻击` 1))))))

(event `Sword_Trace_Stop`
  (`KismetSystemLibrary.K2_ClearAndInvalidateTimerHandle` (stale `Sword_Trace_Start` _returnvalue)))

(event `Sword_Trace_Start`
  (bind _returnvalue (`KismetSystemLibrary.K2_SetTimerDelegate` (delegate `Sword_Trace_Loop`) 0.001 true)))

(event `Sword_Trace_Loop`
  (bind _staticmesh (`/Game/ThirdPerson/Blueprints/BP_MainCharacter.StaticMesh` (`self.Main_character`)))
  (bind _returnvalue (`SceneComponent.K2_GetComponentLocation` _staticmesh))
  (bind _returnvalue_2 (`SceneComponent.K2_GetComponentRotation` _staticmesh))
  (bind (_outhit _returnvalue_3) (`KismetSystemLibrary.SphereTraceSingle` :`Start` (+ _returnvalue (`KismetMathLibrary.GreaterGreater_VectorRotator` (0.0 0.0 50.0) _returnvalue_2)) :`End` (+ _returnvalue (`KismetMathLibrary.GreaterGreater_VectorRotator` (0.0 0.0 -111.0) _returnvalue_2)) :`Radius` 12.0 :`TraceChannel` "TraceTypeQuery1" :`DrawTime` 0.1))
  (if _returnvalue_3
    (bind (_bblockinghit _binitialoverlap _time _distance _location _impactpoint _normal _impactnormal _physmat _hitactor) (`GameplayStatics.BreakHitResult` _outhit))
    (if (`Actor.ActorHasTag` _hitactor "harm")
      (`/Engine/EditorBlueprintResources/StandardMacros.DoOnce` false :!label _label_2
        (:`Completed`
          (`GameplayStatics.ApplyDamage` _hitactor 20.0 null (`self.Main_character`))
          (`GameplayStatics.PlayWorldCameraShake` "/Game/BluePrints/BP_Cam_剑攻击抖动.BP_Cam_剑攻击抖动_C" _location 0.0 2000.0)
          (`GameplayStatics.SpawnEmitterAtLocation` "/Game/VFX/Particles/Blood/P_Blood_Splat_Cone.P_Blood_Splat_Cone" _location (`KismetMathLibrary.MakeRotFromXY` _normal _normal) (0.4 0.4 0.4) true "AutoRelease")
          (`GameplayStatics.PlaySoundAtLocation` "/Game/Audio/剑攻击/MS_Sword_Hit.MS_Sword_Hit" (`Actor.K2_GetActorLocation` (`self.Main_character`)) (struct) 1.0 1.0 0.0 null null null null)
          (`KismetSystemLibrary.Delay` 0.2)
          (goto _label_2 :!via `Reset`))))))

(event `Body_Trace_Stop`
  (`KismetSystemLibrary.K2_ClearAndInvalidateTimerHandle` (stale `Body_Trace_Start` _returnvalue)))

(event `Body_Trace_Start`
  (params (Body_Type :type "/Game/BluePrints/Struct/Enum_身体攻击 Enum" :default "NewEnumerator0"))
  (bind _returnvalue (`KismetSystemLibrary.K2_SetTimerDelegate` (delegate `Body_Trace_loop`) 0.005 true)))

(event `Body_Trace_loop`
  (bind _returnvalue (`SceneComponent.GetSocketLocation` (`Character.Mesh` (`self.Main_character`)) "ball_r"))
  (`KismetSystemLibrary.SphereTraceSingle` :`Start` _returnvalue :`End` _returnvalue :`Radius` 12.0 :`TraceChannel` "TraceTypeQuery1" :`DrawDebugType` "ForDuration" :`DrawTime` 0.1))