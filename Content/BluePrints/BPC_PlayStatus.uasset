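; BPC_PlayStatus is a status component tracking the player's health, stamina, XP and level.
; AddHeart clamps health and flags death at zero, while AddStamina rejects overspending and manages a looping timer, cleared on overfilling, presumably for StaminaAutoRecover.
; That recovery function restores stamina only while the owning BP_ThirdPersonCharacter is not sprinting.
; AddXp loops through multiple level-ups with carryover, each raising the XP threshold linearly and playing sounds.
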(fn `AddHeart`
  (params (Heart :type "Float (double-precision)"))
  (returns (Death :type Boolean))
  (bind _returnvalue (+ (`self.CurHeart`) Heart))
  (if (<= _returnvalue 0.0)
    (set `self.b_death` true)
    (set `self.CurHeart` 0.0)
    (return true)
    (else
      (if (> _returnvalue (`self.MaxHeart`))
        (set `self.CurHeart` (`self.MaxHeart`))
        (else
          (set `self.CurHeart` _returnvalue)))
      (return false))))

(fn `AddLever`
  (`/Engine/EditorBlueprintResources/StandardMacros.IncrementInt` (`self.Lever`)
    (:`  `
      (set `self.MaxXp` (+ (`self.MaxXp`) 150.0))
      (`GameplayStatics.PlaySound2D` "/Game/Audio/UI/Level_up1.Level_up1" 1.0 1.0 0.0 null null)
      (`GameplayStatics.PlaySound2D` "/Game/Audio/UI/Level_up2.Level_up2" 1.0 1.0 0.0 null null))))

(fn `AddMaxHeart`
  (params (Heart :type "Float (double-precision)"))
  (set `self.MaxHeart` (+ Heart (`self.MaxHeart`))))

(fn `AddMaxStamina`
  (params (Stamina :type "Float (double-precision)"))
  (set `self.MaxStamina` (+ Stamina (`self.MaxStamina`))))

(fn `AddStamina`
  (params (Stamina :type "Float (double-precision)"))
  (returns (result :type Boolean))
  (bind _stamina_time_hander (`self.Stamina_time_hander`))
  (bind _returnvalue (+ Stamina (`self.CurStamina`)))
  ;[1 1 1] 如果精力不够，则返回扣除失败
  (if (< _returnvalue 0.0)
    (return false)
    (else
      (if (> _returnvalue (`self.MaxStamina`))
        (set `self.CurStamina` (`self.MaxStamina`))
        (`KismetSystemLibrary.K2_ClearAndInvalidateTimerHandle` _stamina_time_hander)
        (else
          (set `self.CurStamina` _returnvalue)
          (if (`KismetSystemLibrary.K2_IsTimerActiveHandle` _stamina_time_hander)
            _
            (else
              (bind _returnvalue_2 (`KismetSystemLibrary.K2_SetTimerDelegate` (`|CreateDelegate` :!event `StaminaAutoRecover`) 0.1 true))
              (set `self.Stamina_time_hander` _returnvalue_2)
              (return true)))))
      (return true))))

(fn `AddXp`
  (params (InXp :type "Float (double-precision)"))
  (set `self.Xp` (+ InXp (`self.Xp`)))
  (if (>= (`self.Xp`) (`self.MaxXp`)) :!label _label
    (set `self.Xp` (- (`self.Xp`) (`self.MaxXp`)))
    (`self.AddLever`)
    (goto _label)))

(fn `StaminaAutoRecover`
  (bind _asbp_third_person_character (cast `/Game/ThirdPerson/Blueprints/BP_ThirdPersonCharacter` (`self.GetOwner` self)))
  (if (not (`/Game/ThirdPerson/Blueprints/BP_ThirdPersonCharacter.b_sprint` _asbp_third_person_character))
    (`self.AddStamina` 1.0)))