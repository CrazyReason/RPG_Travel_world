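; Equipment component for the main character that handles weapon pickup, the equipment menu and visible gear.
; The interact input sphere-traces from the follow camera, stores a hit BP_Weapon's item data in WeaponSlot and destroys the actor.
; The menu input toggles WB_EquipmentSystem along with cursor and input mode.
; 佩带装备 (equip) sets the character's melee, bow or shield mesh by item type, with no mesh mapped for armor.
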(event Custom|佩带装备
  (params (NewParam :type Struct%20Weapon%20Structure))
  (bind _as_bp_main_character (Variables|Default|GetAs%20BP%20Main%20Character))
  (Components|StaticMesh|SetStaticMesh (Utilities|Select :Index (.类型 NewParam) :NewEnumerator0 (Variables|/Game/ThirdPerson/Blueprints/BP_MainCharacter.BP_MainCharacter_C|GetStaticMesh _as_bp_main_character) :NewEnumerator1 (Variables|/Game/ThirdPerson/Blueprints/BP_MainCharacter.BP_MainCharacter_C|GetStaticMesh_弓 _as_bp_main_character) :NewEnumerator2 0 :NewEnumerator3 (Variables|/Game/ThirdPerson/Blueprints/BP_MainCharacter.BP_MainCharacter_C|GetStaticMesh_盾 _as_bp_main_character)) (.staticmesh NewParam)))

(event Input|EnhancedActionEvents|EnhancedInputActionIA_Interaction
  (params (ActionValue :type Boolean) (ElapsedSeconds :type Float%20%28double-precision%29) (TriggeredSeconds :type Float%20%28double-precision%29) (InputAction :type Input%20Action%20Object%20Reference :default "/Game/ThirdPerson/Input/Actions/IA_Interaction.IA_Interaction"))
  (bind _follow_camera (Variables|Default|GetFollow%20Camera))
  (bind _returnvalue (Transformation|GetWorldLocation _follow_camera))
  (:Started
    (bind (_outhit _returnvalue_2) (Collision|SphereTraceForObjects _returnvalue (+ _returnvalue (* (Math|Vector|GetForwardVector (Transformation|GetWorldRotation _follow_camera)) 1e+03)) 2e+01 (Utilities|Array|MakeArray "ObjectTypeQuery2") false 0 "ForDuration"))
    (if _returnvalue_2
      (bind _asbp_weapon (Utilities|Casting|CastToBP_Weapon (.HitActor (Collision|BreakHitResult _outhit))))
      (CallFunction|AddWeapon (Variables|/Game/BluePrints/Struct/EquipmentSystem/BP_Weapon.BP_Weapon_C|GetItemData _asbp_weapon))
      (Actor|DestroyActor (.HitActor (Collision|BreakHitResult _outhit))))))

(event Input|EnhancedActionEvents|EnhancedInputActionIA_EquipmentMenu
  (params (ActionValue :type Boolean) (ElapsedSeconds :type Float%20%28double-precision%29) (TriggeredSeconds :type Float%20%28double-precision%29) (InputAction :type Input%20Action%20Object%20Reference :default "/Game/ThirdPerson/Input/Actions/IA_EquipmentMenu.IA_EquipmentMenu"))
  (bind _as_bp_main_character (Variables|Default|GetAs%20BP%20Main%20Character))
  (bind _returnvalue (Pawn|GetLocalViewingPlayerController _as_bp_main_character))
  (:Started
    (bind _wb_装备ui显示 (Variables|Default|GetWB_装备UI显示)
      (:then
        (Widget|RemovefromParent _wb_装备ui显示)
        (Variables|Default|SetWB_装备UI显示 0)
        (Variables|/Script/Engine.PlayerController|SetbShowMouseCursor _returnvalue false)
        (Input|SetInputModeGameOnly _returnvalue false))
      (:else
        (bind _returnvalue_2 (UserInterface|CreateWidget "/Game/UI/Weapon/WB_EquipmentSystem.WB_EquipmentSystem_C" _returnvalue))
        (bind _output_get (Variables|Default|SetWB_装备UI显示 _returnvalue_2))
        (UserInterface|Viewport|AddtoViewport _output_get 0)
        (Variables|/Script/Engine.PlayerController|SetbShowMouseCursor _returnvalue true)
        (Input|SetInputModeGameandUI _returnvalue (Variables|Default|GetWB_装备UI显示) "DoNotLock" true false)))))

(event EventBeginPlay
  (bind _asbp_main_character (Utilities|Casting|CastToBP_MainCharacter (Components|GetOwner)))
  (bind _output_get (Variables|Default|SetAs%20BP%20Main%20Character _asbp_main_character))
  (Variables|Default|SetFollow%20Camera (Variables|/Game/ThirdPerson/Blueprints/BP_MainCharacter.BP_MainCharacter_C|GetFollowCamera _output_get)))

(event EventTick
  (params (DeltaSeconds :type Float%20%28single-precision%29)))

(event Input|KeyboardEvents|DebugKeyH
  (params (Key :type Key%20Structure :default "None") (ActionValue :type Input%20Action%20Value%20Structure))
  (:Pressed
    (for _array_element (Variables|Default|GetWeaponSlot)
      (Development|PrintString (Utilities|String|ToString(Name) (.rowname _array_element))))))

(fn AddWeapon
  (params (NewItem :type Data%20Table%20Row%20Handle%20Structure%20%28by%20ref%29))
  (Utilities|Array|Add (Variables|Default|GetWeaponSlot) NewItem))