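; Quest component that holds an owner's quest table and, for the player, tracks accepted quests as references to the giver's component plus quest index.
; Accept, abandon and track write state directly into the giver's table, with a toggled quest window for input.
; On player 0 it creates the HUD and binds kill events that advance class-matched objectives.
; A quest completes unless a matched objective remains short, so unmatched objectives are ignored.
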(event `self.ReceiveBeginPlay`
  (bind _qusettable (`self.QusetTable`))
  (for (_ _array_index) _qusettable
    (setmembers `/Game/BluePrints/Struct/QuestSystem/S_Quest` :`StructRef` (`|GetArrayItem` _qusettable _array_index) :`序号` _array_index))
  (if (== (`self.GetOwner`) (`GameplayStatics.GetPlayerCharacter` 0))
    (bind _returnvalue (`|CreateWidget` "/Game/UI/Quset/WB_QusetHub.WB_QusetHub_C" null self))
    (`UserWidget.AddToViewport` _returnvalue 0)
    (set `self.WB_hub` _returnvalue)
    (bind _asbp_main_character (cast `/Game/ThirdPerson/Blueprints/BP_MainCharacter` (`self.GetOwner`)))
    (add `/Game/ThirdPerson/Blueprints/BP_MainCharacter.击杀` _asbp_main_character (delegate `接受击杀通知`))))

(event `接受击杀通知`
  (params (`被击杀者` :type "Actor Object Reference"))
  (for (_array_element _array_index) (`self.QusetReceive`)
    (set `self.本次任务目标是否完成` true)
    (bind _qusettable (`/Game/BluePrints/BPC_QusetSystem.QusetTable` (break `/Game/BluePrints/Struct/QuestSystem/S_QuestReceive` _array_element)))
    (bind (`_output_序号` `_output_名字` `_output_描述` `_output_主线任务_` `_output_跟踪任务_` `_output_完成_` `_output_接取_` `_output_委托人` `_output_接取者` `_output_任务目标`) (break `/Game/BluePrints/Struct/QuestSystem/S_Quest` (`|GetArrayItem` _qusettable (`.委托人的任务编号_5_8724BC9B4F195D57CA244E967DB8D308` (break `/Game/BluePrints/Struct/QuestSystem/S_QuestReceive` _array_element)))))
    (for (_array_element_2 _array_index_2) `_output_任务目标`
      (bind (`_任务类型` `_目标名称` `_已完成` `_任务量` `_目标种类`) (break `/Game/BluePrints/Struct/QuestSystem/S_Qusest_Target` _array_element_2))
      (if (== `_目标种类` (`GameplayStatics.GetObjectClass` `被击杀者`))
        (bind _returnvalue (+ `_已完成` 1))
        (setmembers `/Game/BluePrints/Struct/QuestSystem/S_Qusest_Target` :`StructRef` (`|GetArrayItem` `_output_任务目标` _array_index_2) :`已完成` _returnvalue)
        (if (not (>= _returnvalue `_任务量`))
          (set `self.本次任务目标是否完成` false))))
    (if (`self.本次任务目标是否完成`)
      (setmembers `/Game/BluePrints/Struct/QuestSystem/S_Quest` :`StructRef` (`|GetArrayItem` _qusettable (`.委托人的任务编号_5_8724BC9B4F195D57CA244E967DB8D308` (break `/Game/BluePrints/Struct/QuestSystem/S_QuestReceive` _array_element))) :`完成?` true)
      (`KismetArrayLibrary.Array_Remove` (`self.QusetReceive`) _array_index)
      (`GameplayStatics.PlaySound2D` "/Game/Audio/UI/Level_up2.Level_up2" 1.0 1.0 0.0 null null)
      (`/Game/UI/Quset/WB_QusetHub.任务完成` (`self.WB_hub`))))
  (`/Game/UI/Quset/WB_QusetHub.界面显示任务` (`self.WB_hub`)))

(event `打开任务系统`
  (params (`任务发放者` :type "/Game/ThirdPerson/Blueprints/BP_MainCharacter Object Reference"))
  (bind _returnvalue (`GameplayStatics.GetPlayerController` 0))
  (bind _returnvalue_2 (`GameplayStatics.GetPlayerController` 0))
  ;[1 1 1] 打开当前的任务列表，优先打开别人的任务，如果没有再打开自家的，接取时，在别人的列表上操作即可
  (if (`self.b_Quset`)
    (`Widget.RemoveFromParent` (`self.wb_Quset`))
    (set `self.b_Quset` false)
    (set `PlayerController.bShowMouseCursor` false _returnvalue_2)
    (`WidgetBlueprintLibrary.SetInputMode_GameOnly` _returnvalue_2)
    (else
      (`/Engine/EditorBlueprintResources/StandardMacros.IsValid` `任务发放者`
        (:`Is Valid`
          (bind _returnvalue_3 (`|CreateWidget` "/Game/UI/Quset/WB_QusetSysteam.WB_QusetSysteam_C" null (`/Game/ThirdPerson/Blueprints/BP_MainCharacter.BPC_QusetSystem` `任务发放者`) self))
          (bind _output_get (set `self.wb_Quset` _returnvalue_3))
          (`UserWidget.AddToViewport` _output_get 0))
        (:`Is Not Valid`
          (bind _returnvalue_4 (`|CreateWidget` "/Game/UI/Quset/WB_QusetSysteam.WB_QusetSysteam_C" null null self))
          (bind _output_get_2 (set `self.wb_Quset` _returnvalue_4))
          (`UserWidget.AddToViewport` _output_get_2 0)))
      (set `self.b_Quset` true)
      (set `PlayerController.bShowMouseCursor` true _returnvalue)
      (`WidgetBlueprintLibrary.SetInputMode_GameAndUIEx` _returnvalue (`self.wb_Quset`)))))

(event `接取任务`
  (params (tar :type "/Game/BluePrints/BPC_QusetSystem Object Reference") (index :type Integer))
  (`KismetArrayLibrary.Array_Add` (`self.QusetReceive`) (make `/Game/BluePrints/Struct/QuestSystem/S_QuestReceive` tar index))
  (setmembers `/Game/BluePrints/Struct/QuestSystem/S_Quest` :`StructRef` (`|GetArrayItem` (`/Game/BluePrints/BPC_QusetSystem.QusetTable` tar) index) :`接取?` true))

(event `放弃任务`
  (params (tar :type "/Game/BluePrints/BPC_QusetSystem Object Reference") (index :type Integer))
  (bind (`_output_委托人` `_output_委托人的任务编号`) (break `/Game/BluePrints/Struct/QuestSystem/S_QuestReceive` (`|GetArrayItem` (`self.QusetReceive`) index)))
  (`/Engine/EditorBlueprintResources/StandardMacros.IsValid` tar
    (:`Is Valid`
      (bind _array_index (`self.寻找任务index` tar index))
      (`KismetArrayLibrary.Array_Remove` (`self.QusetReceive`) _array_index)
      (setmembers `/Game/BluePrints/Struct/QuestSystem/S_Quest` :`StructRef` (`|GetArrayItem` (`/Game/BluePrints/BPC_QusetSystem.QusetTable` tar) index) :`跟踪任务?` false :`接取?` false)
      (bind _wb_hub (`self.WB_hub`)
        (:`then`
          (`/Game/UI/Quset/WB_QusetHub.界面显示任务` _wb_hub))
        (:`else`)))
    (:`Is Not Valid`
      (`/Engine/EditorBlueprintResources/StandardMacros.IsValid` `_output_委托人`
        (:`Is Valid`
          (setmembers `/Game/BluePrints/Struct/QuestSystem/S_Quest` :`StructRef` (`|GetArrayItem` (`/Game/BluePrints/BPC_QusetSystem.QusetTable` `_output_委托人`) `_output_委托人的任务编号`) :`跟踪任务?` false :`接取?` false))
        (:`Is Not Valid`
          _))
      (`KismetArrayLibrary.Array_Remove` (`self.QusetReceive`) index)
      (bind _wb_hub_2 (`self.WB_hub`)
        (:`then`
          (`/Game/UI/Quset/WB_QusetHub.界面显示任务` _wb_hub_2))
        (:`else`)))))

(event `Action`
  (params (tar :type "/Game/BluePrints/BPC_QusetSystem Object Reference") (index :type Integer))
  (bind _output (`|GetArrayItem` (`/Game/BluePrints/BPC_QusetSystem.QusetTable` tar) index))
  (bind (`_output_委托人` `_output_委托人的任务编号`) (break `/Game/BluePrints/Struct/QuestSystem/S_QuestReceive` (`|GetArrayItem` (`self.QusetReceive`) index)))
  (bind _output_2 (`|GetArrayItem` (`/Game/BluePrints/BPC_QusetSystem.QusetTable` `_output_委托人`) `_output_委托人的任务编号`))
  (`/Engine/EditorBlueprintResources/StandardMacros.IsValid` tar
    (:`Is Valid`
      (setmembers `/Game/BluePrints/Struct/QuestSystem/S_Quest` :`StructRef` _output :`跟踪任务?` (not (`.跟踪任务?_13_FF1B031B4E6672AAAB27D9BFFF8C9C88` (break `/Game/BluePrints/Struct/QuestSystem/S_Quest` _output))))
      (bind _wb_hub (`self.WB_hub`)
        (:`then`
          (`/Game/UI/Quset/WB_QusetHub.界面显示任务` _wb_hub))
        (:`else`)))
    (:`Is Not Valid`
      (setmembers `/Game/BluePrints/Struct/QuestSystem/S_Quest` :`StructRef` _output_2 :`跟踪任务?` (not (`.跟踪任务?_13_FF1B031B4E6672AAAB27D9BFFF8C9C88` (break `/Game/BluePrints/Struct/QuestSystem/S_Quest` _output_2))))
      (bind _wb_hub_2 (`self.WB_hub`)
        (:`then`
          (`/Game/UI/Quset/WB_QusetHub.界面显示任务` _wb_hub_2))
        (:`else`)))))

(fn `OnRep_WB_hub`)

(fn `寻找任务index`
  (params (tar :type "Object Object Reference") (index :type Integer))
  (returns (`Array Index` :type Integer))
  (for (_array_element _array_index) (`self.QusetReceive`)
    (if (and (== (break `/Game/BluePrints/Struct/QuestSystem/S_QuestReceive` _array_element) tar) (== (`.委托人的任务编号_5_8724BC9B4F195D57CA244E967DB8D308` (break `/Game/BluePrints/Struct/QuestSystem/S_QuestReceive` _array_element)) index))
      (break)))
  (return _array_index))