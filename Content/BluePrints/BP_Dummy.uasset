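; BP_Dummy is a target character for stealth back assassinations, with a widget shown only while something overlaps its sphere.
; StealthBackAssassin plays the paired knife victim montage, hides the widget, and returns the SkeletalMesh location and actor rotation, presumably for aligning the attacker.
; It also triggers RegDog, which uses separate delays to play a death sound and then turn the mesh into a physics ragdoll.
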(event `self.ReceiveBeginPlay`
  (`KismetSystemLibrary.Delay` 0.01)
  (`SceneComponent.SetVisibility` (`self.Widget`) false false))

(event `RegDog`
  (`|ExecutionSequence`
    (:`then_0`
      (`KismetSystemLibrary.Delay` 2.5)
      (`PrimitiveComponent.SetSimulatePhysics` (`self.Mesh`) true))
    (:`then_1`
      (`KismetSystemLibrary.Delay` 1.8)
      (`GameplayStatics.PlaySoundAtLocation` "/Game/Audio/Grunt/SC_Death.SC_Death" (`self.K2_GetActorLocation`) (struct) 1.0 1.0 0.0 "/Game/Audio/SA_Characters.SA_Characters" null null null))))

(event `self.Sphere.OnComponentBeginOverlap`
  (params (OverlappedComponent :type "PrimitiveComponent Object Reference") (OtherActor :type "Actor Object Reference") (OtherComp :type "PrimitiveComponent Object Reference") (OtherBodyIndex :type Integer) (bFromSweep :type Boolean) (SweepResult :type "HitResult Structure (by ref)"))
  (`SceneComponent.SetVisibility` (`self.Widget`) true false))

(event `self.Sphere.OnComponentEndOverlap`
  (params (OverlappedComponent :type "PrimitiveComponent Object Reference") (OtherActor :type "Actor Object Reference") (OtherComp :type "PrimitiveComponent Object Reference") (OtherBodyIndex :type Integer))
  (`SceneComponent.SetVisibility` (`self.Widget`) false false))

(fn `StealthBackAssassin`
  (returns (location :type "Vector Structure") (Roation :type "Rotator Structure"))
  (`self.PlayAnimMontage` "/Game/Characters/RPG_Characters/Animations/Assassination/Paired_Knife_Stealth_KidneyAndNeck_Vic_Montage.Paired_Knife_Stealth_KidneyAndNeck_Vic_Montage")
  (`self.RegDog`)
  (`SceneComponent.SetVisibility` (`self.Widget`) false false)
  (return (`SceneComponent.K2_GetComponentLocation` (`self.SkeletalMesh`)) (`self.K2_GetActorRotation`)))

(fn `UserConstructionScript`)