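; Dialogue component that shows a conversation line by line, then hands off to the quest system.
; Interaction takes an overlapping BP_MainCharacter as target and reads text from that target's own dialogue component.
; Each call creates or advances a WB_Dialogue widget, resetting the line index only when the target changes.
; After the last line, it removes the widget and opens the owner's BPCQusetSystem for that target.
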(event `与人物交互`
  (set `self.目标` null)
  (for _array_element (`Actor.GetOverlappingActors` (`self.GetOwner`) null)
    (bind _asbp_main_character (cast `/Game/ThirdPerson/Blueprints/BP_MainCharacter` _array_element))
    (set `self.目标` _asbp_main_character)
    (break))
  (`self.打开对话框`))

(event `EnhancedInput|/Game/ThirdPerson/Input/Actions/IA_Interaction`
  (params (ActionValue :type Boolean) (ElapsedSeconds :type "Float (double-precision)") (TriggeredSeconds :type "Float (double-precision)") (InputAction :type "InputAction Object Reference" :default "/Game/ThirdPerson/Input/Actions/IA_Interaction.IA_Interaction")))

(event `打开对话框`
  (`self.对话控件`
    (:`then`
      (bind _bend (`self.切换下一个对话`))
      (if _bend
        (`self.对话结束`)))
    (:`else`
      (bind _returnvalue (`|CreateWidget` "/Game/UI/WB_Dialogue.WB_Dialogue_C"))
      (bind _output_get (set `self.对话控件` _returnvalue))
      (`UserWidget.AddToViewport` _output_get 0)
      (if (not (== (`self.旧的目标`) (`self.目标`)))
        (set `self.旧的目标` (`self.目标`))
        (set `self.当前对话` 0))
      (bind _bend_2 (`self.切换下一个对话`))
      (if _bend_2
        (`self.对话结束`)))))

(event `对话结束`
  (`Widget.RemoveFromParent` (`self.对话控件`))
  (set `self.对话控件` null)
  (bind _asbp_main_character (cast `/Game/ThirdPerson/Blueprints/BP_MainCharacter` (`self.GetOwner`)))
  (`/Game/BluePrints/BPC_QusetSystem.打开任务系统` (`/Game/ThirdPerson/Blueprints/BP_MainCharacter.BPC_QusetSystem` _asbp_main_character) (`self.目标`)))

(fn `切换下一个对话`
  (returns (bEnd :type Boolean))
  (bind `_目标` (`self.目标`)
    (:`then`
      (bind `_对话内容` (`/Game/BluePrints/BPC_DialogueSystem.对话内容` (`/Game/ThirdPerson/Blueprints/BP_MainCharacter.BPC_DialogueSystem` `_目标`)))
      (if (>= (`self.当前对话`) (`KismetArrayLibrary.Array_Length` `_对话内容`))
        (return true)
        (else
          (`TextBlock.SetText` (`/Game/UI/WB_Dialogue.TextBlock_934` (`self.对话控件`)) (`KismetTextLibrary.Conv_StringToText` (`|GetArrayItem` `_对话内容` (`self.当前对话`))))
          (`/Engine/EditorBlueprintResources/StandardMacros.IncrementInt` (`self.当前对话`)
            (:`  `
              (return false))))))
    (:`else`
      (return true))))