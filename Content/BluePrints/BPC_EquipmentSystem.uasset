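; BPC_EquipmentSystem is an equipment component for BP_MainCharacter that handles the equipment menu and shows equipped items on the character.
; The IA_EquipmentMenu input toggles the WB_EquipmentSystem widget, switching mouse cursor and input mode with it.
; The equip event (佩带装备) routes an item's static mesh by type to the character's melee, bow or shield mesh component, with armor unassigned.
; AddWeapon appends items to WeaponSlot.
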(event `self.ReceiveBeginPlay`
  (bind _asbp_main_character (cast `/Game/ThirdPerson/Blueprints/BP_MainCharacter` (`self.GetOwner`)))
  (set `self.As BP Main Character` _asbp_main_character))

(event `EnhancedInput|/Game/ThirdPerson/Input/Actions/IA_EquipmentMenu`
  (params (ActionValue :type Boolean) (ElapsedSeconds :type "Float (double-precision)") (TriggeredSeconds :type "Float (double-precision)") (InputAction :type "InputAction Object Reference" :default "/Game/ThirdPerson/Input/Actions/IA_EquipmentMenu.IA_EquipmentMenu"))
  (bind _returnvalue (`Pawn.GetLocalViewingPlayerController` (`self.As BP Main Character`)))
  (:`Started`
    (bind `_wb_装备ui显示` (`self.WB_装备UI显示`)
      (:`then`
        (`Widget.RemoveFromParent` `_wb_装备ui显示`)
        (set `self.WB_装备UI显示` null)
        (set `PlayerController.bShowMouseCursor` false _returnvalue)
        (`WidgetBlueprintLibrary.SetInputMode_GameOnly` _returnvalue))
      (:`else`
        (bind _returnvalue_2 (`|CreateWidget` "/Game/UI/Weapon/WB_EquipmentSystem.WB_EquipmentSystem_C" _returnvalue))
        (bind _output_get (set `self.WB_装备UI显示` _returnvalue_2))
        (`UserWidget.AddToViewport` _output_get 0)
        (set `PlayerController.bShowMouseCursor` true _returnvalue)
        (`WidgetBlueprintLibrary.SetInputMode_GameAndUIEx` _returnvalue (`self.WB_装备UI显示`))))))

(event `佩带装备`
  (params (Wepon :type "/Game/BluePrints/Struct/EquipmentSystem/Struct_Weapon Structure"))
  (bind _as_bp_main_character (`self.As BP Main Character`))
  (`StaticMeshComponent.SetStaticMesh` (select `/Game/BluePrints/Struct/EquipmentSystem/Enum_武器种类` `Wepon_类型_18_3E04934649472857052E6E8972B0527C` :`NewEnumerator0` (`/Game/ThirdPerson/Blueprints/BP_MainCharacter.StaticMesh` _as_bp_main_character) :`NewEnumerator1` (`/Game/ThirdPerson/Blueprints/BP_MainCharacter.StaticMesh_弓` _as_bp_main_character) :`NewEnumerator3` (`/Game/ThirdPerson/Blueprints/BP_MainCharacter.StaticMesh_盾` _as_bp_main_character)) Wepon_staticmesh_13_90BABFD645B41DD404572689CA213210))

(fn `AddWeapon`
  (params (NewItem :type "DataTableRowHandle Structure (by ref)"))
  (`KismetArrayLibrary.Array_Add` (`self.WeaponSlot`) NewItem))