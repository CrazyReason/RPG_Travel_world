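; BP_Dummy is a dummy enemy character that takes damage and can be stealth-assassinated from behind.
; AnyDamage plays a random montage, then launches it along the causer's forward vector and updates BPCPlayStatus health, ragdolling it when AddHeart returns true.
; StealthBackAssassin plays the paired victim montage, triggers delayed ragdoll and death sound, and returns a location and rotation.
; A camera-facing health widget reads BPCPlayStatus, while a sphere overlap toggles a second widget.
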(event `self.ReceiveBeginPlay`
  (`KismetSystemLibrary.Delay` 0.01)
  (`SceneComponent.SetVisibility` (`self.Widget`) false false)
  (bind _aswb_status (cast `/Game/UI/WB_Dummy_Hp` (`WidgetComponent.GetWidget` (`self.Widget_Status`))))
  (set `/Game/UI/WB_Dummy_Hp.PlayStatus` (`self.BPC_PlayStatus`) _aswb_status))

(event `self.ReceiveTick`
  (params (DeltaSeconds :type "Float (single-precision)"))
  (`SceneComponent.K2_SetWorldRotation` (`self.Widget_Status`) (`KismetMathLibrary.FindLookAtRotation` (`SceneComponent.K2_GetComponentLocation` (`self.Widget_Status`)) (`SceneComponent.K2_GetComponentLocation` (`PlayerCameraManager.TransformComponent` (`GameplayStatics.GetPlayerCameraManager` 0)))) false false))

(event `RegDog`
  (`|ExecutionSequence`
    (:`then_0`
      (`KismetSystemLibrary.Delay` 2.5)
      (`PrimitiveComponent.SetSimulatePhysics` (`self.Mesh`) true))
    (:`then_1`
      (`KismetSystemLibrary.Delay` 1.8)
      (`GameplayStatics.PlaySoundAtLocation` "/Game/Audio/Grunt/SC_Death.SC_Death" (`self.K2_GetActorLocation`) (struct) 1.0 1.0 0.0 "/Game/Audio/SA_Characters.SA_Characters" null null null))))

(event `self.Sphere.OnComponentBeginOverlap`
  (params (OverlappedComponent :type "PrimitiveComponent Object Reference") (OtherActor :type "Actor Object Reference") (OtherComp :type "PrimitiveComponent Object Reference") (OtherBodyIndex :type Integer) (bFromSweep :type Boolean) (SweepResult :type "HitResult Structure (by ref)"))
  (`SceneComponent.SetVisibility` (`self.Widget`) true false))

(event `self.Sphere.OnComponentEndOverlap`
  (params (OverlappedComponent :type "PrimitiveComponent Object Reference") (OtherActor :type "Actor Object Reference") (OtherComp :type "PrimitiveComponent Object Reference") (OtherBodyIndex :type Integer))
  (`SceneComponent.SetVisibility` (`self.Widget`) false false))

(event `self.ReceiveAnyDamage`
  (params (Damage :type "Float (single-precision)") (DamageType :type "DamageType Object Reference") (InstigatedBy :type "Controller Object Reference") (DamageCauser :type "Actor Object Reference"))
  (`|PlayMontage` (`self.Mesh`) (`|GetArrayItem` (`self.Montage to Play`) (`KismetMathLibrary.RandomIntegerInRange` 0 1))
    (:`then`
      (`self.LaunchCharacter` (* (`self.GetActorForwardVector` DamageCauser) 700.0))
      (`GameplayStatics.PlaySoundAtLocation` "/Game/Audio/Grunt/Death2.Death2" (`self.K2_GetActorLocation`) (struct) 1.0 (`KismetMathLibrary.RandomFloatInRange` -1.2 1.5) 0.0 "/Game/Audio/SA_Characters.SA_Characters" null null null)
      (bind _death (`/Game/BluePrints/BPC_PlayStatus.AddHeart` (`self.BPC_PlayStatus`) (- 0.0 Damage)))
      (if _death
        (`PrimitiveComponent.SetSimulatePhysics` (`self.Mesh`) true)
        (`GameplayStatics.PlaySoundAtLocation` "/Game/Audio/Grunt/SC_Death.SC_Death" (`self.K2_GetActorLocation`) (struct) 1.0 1.0 0.0 "/Game/Audio/SA_Characters.SA_Characters" null null null)
        (`SceneComponent.SetVisibility` (`self.Widget_Status`) false false)))))

(fn `StealthBackAssassin`
  (returns (location :type "Vector Structure") (Roation :type "Rotator Structure"))
  (`self.PlayAnimMontage` "/Game/Characters/RPG_Characters/Animations/Assassination/Paired_Knife_Stealth_KidneyAndNeck_Vic_Montage.Paired_Knife_Stealth_KidneyAndNeck_Vic_Montage")
  (`self.RegDog`)
  (`SceneComponent.SetVisibility` (`self.Widget`) false false)
  (return (`SceneComponent.K2_GetComponentLocation` (`self.SkeletalMesh`)) (`self.K2_GetActorRotation`)))

(fn `UserConstructionScript`)