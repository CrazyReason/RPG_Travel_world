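; Dummy AI NPC that idles in a wander state and offers a task prompt.
; On BeginPlay it links play status to its HP widget, then writes the wander state to the Blackboard and spawns a visible trigger sphere ahead.
; Any overlap flashes "[E] accept task" and sets the stay-in-place key, reset to its default after a delay or on cursor-over end.
; Tick turns both widgets toward the player camera.
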(event `切换活动状态`
  (params (`活动状态` :type "/Game/BluePrints/Struct/Enum_活动状态 Enum" :default "NewEnumerator0"))
  (bind _returnvalue (enumliteral `/Game/BluePrints/Struct/Enum_活动状态` `活动状态`))
  (`BlackboardComponent.SetValueAsEnum` (`AIBlueprintHelperLibrary.GetBlackboard` null) "活动状态" _returnvalue)
  (switch `/Game/BluePrints/Struct/Enum_活动状态` _returnvalue
    (:`NewEnumerator0`
      (`BlackboardComponent.SetValueAsBool` (`AIBlueprintHelperLibrary.GetBlackboard` null) "呆在原地?" (`self.呆在原地?`))
      (bind _returnvalue_2 (`AddComponent|NODE_AddSphereComponent-0` :`self` self :`RelativeTransform` (`KismetMathLibrary.MakeTransform` (60.0 0.0 0.0))))
      (`SphereComponent.SetSphereRadius` _returnvalue_2 80.0 true)
      (`SceneComponent.SetHiddenInGame` _returnvalue_2 false false)
      (add `PrimitiveComponent.OnComponentBeginOverlap` _returnvalue_2 (delegate `进入任务区`))
      (add `PrimitiveComponent.OnEndCursorOver` _returnvalue_2 (delegate `离开任务区`)))))

(event `离开任务区`
  (params (TouchedComponent :type "PrimitiveComponent Object Reference"))
  (`BlackboardComponent.SetValueAsBool` (`AIBlueprintHelperLibrary.GetBlackboard` null) "呆在原地?" (or false (`self.呆在原地?`))))

(event `进入任务区`
  (params (OverlappedComponent :type "PrimitiveComponent Object Reference") (OtherActor :type "Actor Object Reference") (OtherComp :type "PrimitiveComponent Object Reference") (OtherBodyIndex :type Integer) (bFromSweep :type Boolean) (SweepResult :type "HitResult Structure (by ref)"))
  (`self.显示当前状态` "[E] 接取任务")
  (`BlackboardComponent.SetValueAsBool` (`AIBlueprintHelperLibrary.GetBlackboard` null) "呆在原地?" (or true (`self.呆在原地?`)))
  (`KismetSystemLibrary.Delay` 30.0)
  (`self.离开任务区` null))

(event `self.ReceiveBeginPlay`
  (`parent.ReceiveBeginPlay`)
  (bind _aswb_dummy_hp (cast `/Game/UI/WB_Dummy_Hp` (`WidgetComponent.GetWidget` (`self.Widget_boxy`))))
  (set `/Game/UI/WB_Dummy_Hp.PlayStatus` (`self.BPC_PlayStatus`) _aswb_dummy_hp)
  (`self.切换活动状态` "NewEnumerator0"))

(event `self.ReceiveTick`
  (params (DeltaSeconds :type "Float (single-precision)"))
  (bind _widget_boxy (`self.Widget_boxy`))
  (`parent.ReceiveTick` DeltaSeconds)
  (`SceneComponent.K2_SetWorldRotation` _widget_boxy (`KismetMathLibrary.FindLookAtRotation` (`SceneComponent.K2_GetComponentLocation` _widget_boxy) (`SceneComponent.K2_GetComponentLocation` (`PlayerCameraManager.TransformComponent` (`GameplayStatics.GetPlayerCameraManager` 0)))) false false)
  (`SceneComponent.K2_SetWorldRotation` (`self.Widget_Status`) (`KismetMathLibrary.FindLookAtRotation` (`SceneComponent.K2_GetComponentLocation` _widget_boxy) (`SceneComponent.K2_GetComponentLocation` (`PlayerCameraManager.TransformComponent` (`GameplayStatics.GetPlayerCameraManager` 0)))) false false))

(event `显示当前状态`
  (params (TXT :type Text))
  (bind _widget_status (`self.Widget_Status`))
  (bind _aswb_dummy_status (cast `/Game/UI/WB_Dummy_Status` (`WidgetComponent.GetWidget` (`self.Widget_Status`))))
  (set `/Game/UI/WB_Dummy_Status.txt` TXT _aswb_dummy_status)
  (`SceneComponent.SetVisibility` _widget_status true false)
  (`KismetSystemLibrary.RetriggerableDelay` 5.0)
  (`SceneComponent.SetVisibility` _widget_status false false))

(fn `UserConstructionScript`
  (`parent.UserConstructionScript`))