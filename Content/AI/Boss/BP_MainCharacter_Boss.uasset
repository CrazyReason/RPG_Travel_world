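; Boss character Blueprint that enters combat as soon as play begins.
; BeginPlay runs the parent logic, then calls 进入战斗状态 (enter combat state), which creates a WB_Boss_Hp widget, adds it to the viewport and hands it the BPCPlayStatus reference.
; It then sets the blackboard's 活动状态 (activity state) enum key.
; Tick and overlap events are disabled, and construction only calls the parent.
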(event `self.ReceiveBeginPlay`
  (`parent.ReceiveBeginPlay`)
  (`self.进入战斗状态`)
  (`BlackboardComponent.SetValueAsEnum` (`AIBlueprintHelperLibrary.GetBlackboard` null) "活动状态" (enumliteral `/Game/BluePrints/Struct/Enum_活动状态` "NewEnumerator1")))

(event `进入战斗状态`
  (bind _returnvalue (`|CreateWidget` "/Game/UI/WB_Boss_Hp.WB_Boss_Hp_C"))
  (`UserWidget.AddToViewport` _returnvalue 0)
  (set `/Game/UI/WB_Boss_Hp.PlayStatus` (`self.BPC_PlayStatus`) _returnvalue))

(fn `UserConstructionScript`
  (`parent.UserConstructionScript`))