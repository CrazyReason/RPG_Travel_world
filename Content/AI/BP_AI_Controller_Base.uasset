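; Base AI controller that starts the BT_AI behavior tree and feeds sight and hearing perception into its Blackboard.
; Each perception update goes through separate handlers that filter by sense class.
; Sight sets TagActor to the seen actor and clears it when sensing fails.
; Successful hearing stores the noise location and has the controlled BP_MainCharacter_Dummy display a "heard something" status.
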(event `self.ReceiveBeginPlay`
  (`self.RunBehaviorTree` "/Game/AI/BT_AI.BT_AI"))

(event `self.AIPerception.OnTargetPerceptionUpdated`
  (params (Actor :type "Actor Object Reference") (Stimulus :type "AIStimulus Structure"))
  (`self.视觉处理` Actor Stimulus)
  (`self.听觉处理` Actor Stimulus))

(fn `UserConstructionScript`)

(fn `听觉处理`
  (params (InputPin :type "Object Object Reference") (AIStimulus :type "AIStimulus Structure (by ref)"))
  (bind (_age _expirationage _strength _stimuluslocation _receiverlocation _tag _bsuccessfullysensed) (break `AIStimulus` AIStimulus))
  (bind _returnvalue (`AIPerceptionSystem.GetSenseClassForStimulus` AIStimulus))
  (if (== _returnvalue "/Script/AIModule.AISense_Hearing")
    (if _bsuccessfullysensed
      (`BlackboardComponent.SetValueAsVector` (`AIBlueprintHelperLibrary.GetBlackboard` null) "听到声音的地方" _stimuluslocation)
      (bind _asbp_main_character_dummy (cast `/Game/AI/XiaoBin/BP_MainCharacter_Dummy` (`self.K2_GetPawn`)))
      (`/Game/AI/XiaoBin/BP_MainCharacter_Dummy.显示状态` _asbp_main_character_dummy "听到动静"))))

(fn `视觉处理`
  (params (Actor :type "Object Object Reference") (AIStimulus :type "AIStimulus Structure (by ref)"))
  (bind _returnvalue (`AIBlueprintHelperLibrary.GetBlackboard` null))
  (bind _returnvalue_2 (`AIPerceptionSystem.GetSenseClassForStimulus` AIStimulus))
  (if (== _returnvalue_2 "/Script/AIModule.AISense_Sight")
    (if (`.bSuccessfullySensed` (break `AIStimulus` AIStimulus))
      (`BlackboardComponent.SetValueAsObject` _returnvalue "TagActor" Actor)
      (else
        (`BlackboardComponent.SetValueAsObject` _returnvalue "TagActor" null)))))